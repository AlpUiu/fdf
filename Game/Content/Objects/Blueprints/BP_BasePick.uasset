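; BP_BasePick is a base Blueprint for objects that can be picked up and dropped.
; On BeginPlay, the Hang flag decides whether the static mesh stays fixed or simulates physics.
; Pick turns off mesh physics and actor collision, and Drop turns both back on.
; The Blueprint only toggles these states and contains no attachment or movement logic.
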(event `self.ReceiveBeginPlay`
  (bind _staticmesh (`self.StaticMesh`))
  (if (`self.Hang?`)
    (`PrimitiveComponent.SetSimulatePhysics` _staticmesh false)
    (else
      (`PrimitiveComponent.SetSimulatePhysics` _staticmesh true))))

(event `Pick`
  (`PrimitiveComponent.SetSimulatePhysics` (`self.StaticMesh`) false)
  (`self.SetActorEnableCollision` false))

(event `Drop`
  (`PrimitiveComponent.SetSimulatePhysics` (`self.StaticMesh`) true)
  (`self.SetActorEnableCollision` true))

(fn `UserConstructionScript`)